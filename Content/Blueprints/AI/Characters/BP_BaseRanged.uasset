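; Base Blueprint for ranged AI characters that shoot at their current target from afar and melee it up close.
; In the Attack state, EvaluateState checks target distance against a close-combat range to pick MeleeAttack or Shoot.
; Shoot spawns a projectile at the fire point, initializes it with random damage, knockback and direction to the target, then starts a timer-based cooldown.
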(fn `EvaluateState`
  (`self.SwitchState`
    (:`Attack`
      (bind _inrange (`self.IsInCloseRange`))
      (if _inrange
        (`self.MeleeAttack`)
        (else
          (`self.Shoot`))))))

(fn `IsInCloseRange`
  (returns (inRange :type Boolean))
  (locals (distance :type "Float (double-precision)"))
  (`/Engine/EditorBlueprintResources/StandardMacros.IsValid` (`self._CurrentTarget`)
    (:`Is Valid`
      (bind _output_get (set `local.distance` (`KismetMathLibrary.Vector_Distance` (`self.K2_GetActorLocation` (`self._CurrentTarget`)) (`self.K2_GetActorLocation`))))
      (if (<= _output_get (`self._closeCombatRange`))
        (return true)
        (else
          (return false))))
    (:`Is Not Valid`
      (return false))))

(fn `ResetRangedAttackCooldown`
  (set `self._canRangeAttack` true))

(fn `Shoot`
  (locals (dmg :type "Float (double-precision)") (dirToTarget :type "Vector Structure"))
  (if (`self._canRangeAttack`)
    (set `local.dmg` (`KismetMathLibrary.RandomFloatInRange` (`self.MinDamage`) (`self.MaxDamage`)))
    (set `local.dirToTarget` (`KismetMathLibrary.GetDirectionUnitVector` (`self.K2_GetActorLocation`) (`self.K2_GetActorLocation` (`self._CurrentTarget`))))
    (bind _returnvalue (`|SpawnActorFromClass` (`self.projectileType`) (`KismetMathLibrary.MakeTransform` (`SceneComponent.K2_GetComponentLocation` (`self.FirePoint`)) (`SceneComponent.K2_GetComponentRotation` (`self.FirePoint`))) "Undefined" "OverrideRootScale" null null))
    (bind _asbp_base_projectile (cast `/Game/Blueprints/Weapon/Enemy/BP_BaseProjectile` _returnvalue))
    (`/Game/Blueprints/Weapon/Enemy/BP_BaseProjectile.InitProjectile` _asbp_base_projectile (`self._projectileSpeed`) (`self._knockBack`) (`local.dmg`) self (`local.dirToTarget`))
    (set `self._canRangeAttack` false)
    (bind _returnvalue_2 (`KismetSystemLibrary.K2_SetTimer` null "ResetRangedAttackCooldown" (`self._RangedAttackCooldown`)))
    (set `self._RangedAttackCooldownHandle` _returnvalue_2)
    (`KismetSystemLibrary.PrintString` "Shooting" true true (struct :`R` 0.996818 :`G` 1.0 :`A` 1.0))))

(fn `UserConstructionScript`
  (`parent.UserConstructionScript`))
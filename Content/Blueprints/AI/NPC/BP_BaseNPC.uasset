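; Base NPC character that wanders, chases or attacks a target, with health, team and an attached weapon.
; An enum state sets walk speed, a looping timer switches Chase and Attack by range, and Tick calls the melee attack.
; Damage arrives through I_Damageable, and on death the NPC notifies its attacker and destroys itself.
; The melee damage and cooldown nodes are disconnected, so attacks currently deal no damage.
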(event `self.ReceiveBeginPlay`
  (`self.InitNPC`))

(event `/Game/Blueprints/Interfaces/I_Damageable.TargetDestroyed`
  (`self.SetNewAIState` "NewEnumerator0")
  (`self.SetNPCtarget` null))

(event `self.ReceiveTick`
  (params (DeltaSeconds :type "Float (single-precision)"))
  (`self.EvaluateState`))

(event `/Game/Blueprints/Interfaces/I_Damageable.Damage`
  (params (Damage :type "Float (single-precision)") (KnockBack :type "Float (single-precision)") (InterfacingActor :type "Actor Object Reference"))
  (`self.DamageNPC` Damage)
  (bind _isdead (`self.IsDead`))
  (if _isdead
    (bind _asi_damageable (cast `/Game/Blueprints/Interfaces/I_Damageable` InterfacingActor)
      (:`then`
        (`/Game/Blueprints/Interfaces/I_Damageable.TargetDestroyed` _asi_damageable))
      (:`CastFailed`
        _))
    (`self.K2_DestroyActor`)))

(fn `DamageNPC`
  (params (damage :type "Float (double-precision)"))
  (bind _output_get (set `self._currHealth` (- (`self._currHealth`) damage)))
  (`KismetSystemLibrary.PrintString` (`KismetTextLibrary.Conv_TextToString` (`|FormatText` "Npc Health:{Current Health }" _output_get)) true true (struct :`R` 1.0 :`B` 0.953373 :`A` 1.0)))

(fn `EvaluateState`
  (`self.SwitchState`
    (:`Attack`
      (`self.MeleeAttack`))))

(fn `GetCurrentAIState`
  (returns (currState :type "/Game/Blueprints/AI/DataStructures/E_AIstates Enum"))
  (return (`self._currState`)))

(fn `GetCurrentTarget`
  (returns (isValid :type Boolean) (_CurrentTarget :type "Actor Object Reference"))
  ;[1 1 1] Checks if their is a current target if there isn't don't return and indicate it's not valid
  (`/Engine/EditorBlueprintResources/StandardMacros.IsValid` (`self._CurrentTarget`)
    (:`Is Valid`
      (return true (`self._CurrentTarget`)))
    (:`Is Not Valid`
      (return false null))))

(fn `GetCurrentTargetLocation`
  (returns (ReturnValue :type "Vector Structure"))
  (bind __currenttarget (`self._CurrentTarget`))
  (`/Engine/EditorBlueprintResources/StandardMacros.IsValid` __currenttarget
    (:`Is Valid`
      (return (`self.K2_GetActorLocation` __currenttarget)))))

(fn `I_GetMesh`
  (returns (SkeletalMesh :type "SkeletalMeshComponent Object Reference"))
  (return (`self.Mesh`)))

(fn `I_GetTeam`
  (returns (ETeam :type "/Game/Enums/ETeam Enum"))
  (return (`self.Team`)))

(fn `I_GetWeaponEquipped`
  (returns (WeaponEquipped :type "Actor Object Reference"))
  (return (`ChildActorComponent.ChildActor` (`self.Weapon`))))

(fn `InitNewState`
  (bind __wanderdata_wanderspeed (break `/Game/Blueprints/AI/DataStructures/S_WanderData` (`self._WanderData`)))
  (bind __chasedata_chasespeed (break `/Game/Blueprints/AI/DataStructures/S_ChaseData` (`self._ChaseData`)))
  (`self.SwitchState`
    (:`Wander`
      (set `CharacterMovementComponent.MaxWalkSpeed` __wanderdata_wanderspeed (`self.CharacterMovement`)))
    (:`Chase`
      (set `CharacterMovementComponent.MaxWalkSpeed` __chasedata_chasespeed (`self.CharacterMovement`)))))

(fn `InitNPC`
  (bind __wanderdata_wanderspeed (break `/Game/Blueprints/AI/DataStructures/S_WanderData` (`self._WanderData`)))
  (bind __chasedata_chasespeed (break `/Game/Blueprints/AI/DataStructures/S_ChaseData` (`self._ChaseData`)))
  (`self.SwitchState`
    (:`Wander`
      (set `CharacterMovementComponent.MaxWalkSpeed` __wanderdata_wanderspeed (`self.CharacterMovement`)))
    (:`Chase`
      (set `CharacterMovementComponent.MaxWalkSpeed` __chasedata_chasespeed (`self.CharacterMovement`))))
  (set `self._currHealth` (`self._maxHealth`))
  (bind _asbase_npc_aicontroller (cast `/Game/Blueprints/AI/NPC/BaseNPC_AIController` (`self.GetController`)))
  (`/Game/Blueprints/AI/NPC/BaseNPC_AIController.InitController` _asbase_npc_aicontroller)
  (bind _returnvalue (`KismetSystemLibrary.K2_SetTimer` null "ProcessAI" (`self._AiTickRate`) true))
  (set `self._AiTickTimer` _returnvalue))

(fn `IsDead`
  (returns (isDead :type Boolean))
  (if (<= (`self._currHealth`) 0.0)
    (return true)
    (else
      (return false))))

(fn `IsInRange`
  (returns (inRange :type Boolean))
  (locals (distance :type "Float (double-precision)"))
  (bind (__chasedata_chasespeed __chasedata_attackrange) (break `/Game/Blueprints/AI/DataStructures/S_ChaseData` (`self._ChaseData`)))
  (`/Engine/EditorBlueprintResources/StandardMacros.IsValid` (`self._CurrentTarget`)
    (:`Is Valid`
      (bind _output_get (set `local.distance` (`KismetMathLibrary.Vector_Distance` (`self.K2_GetActorLocation` (`self._CurrentTarget`)) (`self.K2_GetActorLocation`))))
      (if (<= _output_get __chasedata_attackrange)
        (return true)
        (else
          (return false))))
    (:`Is Not Valid`
      (return false))))

(fn `KillNPC`)

(fn `MeleeAttack`
  (locals (dmg :type "Float (double-precision)"))
  (if (`self._canMeleeAttack`)
    (set `local.dmg` (`KismetMathLibrary.RandomFloatInRange` (`self.MinDamage`) (`self.MaxDamage`)))
    (`/Engine/EditorBlueprintResources/StandardMacros.IsValid` (`self._CurrentTarget`)
      (:`Is Not Valid`
        (`self.SetNewAIState` "NewEnumerator0")))))

(fn `ProcessAI`
  (`self.SwitchState`
    (:`Chase`
      (bind _inrange (`self.IsInRange`))
      (if _inrange
        (`self.SetNewAIState` "NewEnumerator2")))
    (:`Attack`
      (bind _inrange_2 (`self.IsInRange`))
      (if (not _inrange_2)
        (`self.SetNewAIState` "NewEnumerator1")))))

(fn `ResetMeleeAttackCooldown`
  (set `self._canMeleeAttack` true))

(fn `SetNewAIState`
  (params (currState :type "/Game/Blueprints/AI/DataStructures/E_AIstates Enum" :default "NewEnumerator0"))
  (set `self._currState` currState)
  (`self.SwitchState`
    (:`Wander`
      ;[1 1 1] If wander just begin to wander
      (`self.OnNewAIState` (`self._currState`))
      (`self.InitNewState`))
    (:`Chase`
      ;[1 1 1] If chase or attack check if there is a valid target
      (`/Engine/EditorBlueprintResources/StandardMacros.IsValid` (`self._CurrentTarget`) :!label _label
        (:`Is Valid`
          (`self.OnNewAIState` (`self._currState`))
          (`self.InitNewState`))
        (:`Is Not Valid`
          ;[1 1 1] If not valid begin to wander
          (`self.SetNewAIState` "NewEnumerator0"))))
    (:`Attack`
      (goto _label))
    (:`Idle`
      ;[1 1 1] If idle just be idle
      (`self.OnNewAIState` (`self._currState`))
      (`self.InitNewState`))))

(fn `SetNPCtarget`
  (params (_CurrentTarget :type "Actor Object Reference"))
  (set `self._CurrentTarget` _CurrentTarget))

(fn `UserConstructionScript`
  (`SceneComponent.K2_AttachToComponent` (`self.Weapon`) (`self.Mesh`) "Socket_Weapon" "KeepRelative" "KeepRelative" "KeepRelative" true))
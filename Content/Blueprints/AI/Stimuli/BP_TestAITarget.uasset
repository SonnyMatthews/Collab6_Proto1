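; BP_TestAITarget is a destructible test target for AI, with a simple health pool.
; It sets current health to max on BeginPlay, then subtracts incoming amounts in its Damage event and prints the remaining health on screen.
; When health reaches zero or below, it sends TargetDestroyedMessage back to the actor passed in with the damage, then destroys itself.
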(event `self.ReceiveBeginPlay`
  (set `self.currentHealth` (`self.maxHealth`)))

(event `/Game/Blueprints/Interfaces/I_Damageable.Damage`
  (params (Damage :type "Float (single-precision)") (KnockBack :type "Float (single-precision)") (InterfacingActor :type "Actor Object Reference"))
  (bind _output_get (set `self.currentHealth` (- (`self.currentHealth`) Damage)))
  (`KismetSystemLibrary.PrintString` (`KismetStringLibrary.Conv_DoubleToString` _output_get) true true (struct :`R` 1.0 :`G` 0.131315 :`A` 1.0))
  (if (<= _output_get 0.0)
    (message `/Game/Blueprints/Interfaces/I_Damageable.TargetDestroyed` InterfacingActor)
    (`self.K2_DestroyActor`)))

(fn `UserConstructionScript`)
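; BP_Door is a door that sinks 300 units downward in a short camera cutscene when its ITrigger event fires.
; It slows the player pawn's CustomTimeDilation and blends the view to the door itself, then a timeline lerps the actor's location without sweep.
; After a pause, it casts the pawn to Pawn_Character, blends back to its PawnCamera and restores normal pawn time.
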(event `/Game/Blueprints/Interfaces/I_Trigger.I_Trigger`
  (bind _returnvalue (`GameplayStatics.GetPlayerController` 0))
  (bind _returnvalue_2 (`GameplayStatics.GetPlayerController` 0))
  (set `Actor.CustomTimeDilation` 0.2 (`Controller.K2_GetPawn` _returnvalue_2))
  (`PlayerController.SetViewTargetWithBlend` _returnvalue_2 self 1.0 "VTBlend_Linear" 0.0 false)
  (`KismetSystemLibrary.Delay` 1.0)
  (set `self.StartLoc` (`self.K2_GetActorLocation`))
  (set `self.TargetLoc` (- (`self.K2_GetActorLocation`) (0.0 0.0 300.0)))
  (bind (_direction _newtrack_2) (`Timeline|Timeline_0` :!via `PlayFromStart`)
    (:`Update`
      (`self.K2_SetActorLocation` (`KismetMathLibrary.VLerp` (`self.StartLoc`) (`self.TargetLoc`) _newtrack_2)))
    (:`Finished`
      (`KismetSystemLibrary.Delay` 2.0)
      (bind _aspawn_character (cast `/Game/Blueprints/Pawn/Pawn_Character` (`Controller.K2_GetPawn` _returnvalue)))
      (`PlayerController.SetViewTargetWithBlend` _returnvalue (`/Game/Blueprints/Pawn/Pawn_Character.Pawn_Camera` _aspawn_character) 1.0 "VTBlend_Linear" 0.0 false)
      (set `Actor.CustomTimeDilation` 1.0 (`Controller.K2_GetPawn` _returnvalue)))))

(fn `UserConstructionScript`)
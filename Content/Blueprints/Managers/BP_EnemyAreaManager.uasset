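; Enemy area manager that spawns a configured set of enemies and fires triggers once they are all destroyed.
; On BeginPlay it spawns each SpawnedEnemy type at the target point of the same index, mapping the enum to base melee or ranged Blueprints.
; Spawned enemies have OnDestroyed bound and are tracked in EnemyList; when the death handler empties it, each TriggerTarget receives an ITriggerMessage interface call.
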(event `self.ReceiveBeginPlay`
  (for (_array_element _array_index) (`self.SpawnedEnemy`)
    (`self.Spawn Enemy` _array_element (`|GetArrayItem` (`self.Enemy Spawn Locations`) _array_index))))

(event `EnemyDeath`
  (params (DestroyedActor :type "Actor Object Reference"))
  ;[1 1 1] Bind enemy On Death this event
  (`KismetArrayLibrary.Array_RemoveItem` (`self.Enemy List`) DestroyedActor) ; Removes enemy from list
  (`/Engine/EditorBlueprintResources/StandardMacros.IsValid` (`|GetArrayItem` (`self.Enemy List`)) ; Checks if the first element in the array exists
    (:`Is Not Valid`
      (for _array_element (`self.TriggerTargets`)
        (message `/Game/Blueprints/Interfaces/I_Trigger.I_Trigger` _array_element))
      (`KismetSystemLibrary.PrintString` "TRIGGED"))))

(fn `Spawn Enemy`
  (params (SpawnedType :type "/Game/Enums/Enum_EnemyType Enum" :default "NewEnumerator0") (Location :type "TargetPoint Object Reference"))
  (locals (`Local Transform` :type "Transform Structure"))
  (set `local.Local Transform` (`self.GetTransform` Location)) ; Saves Location of Target Point
  (switch `/Game/Enums/Enum_EnemyType` SpawnedType ; Spawns a different Unit based on enum
    (:`NewEnumerator0`
      ;[1 1 1] Spawns Enemy
      (bind _returnvalue (`|SpawnActorFromClass` "/Game/Blueprints/AI/Characters/BP_BaseMelee.BP_BaseMelee_C" (`local.Local Transform`) "Undefined" "OverrideRootScale" null null))
      ;[1 1 1] Binds on Death to Manager
      (add `self.OnDestroyed` _returnvalue (`|CreateDelegate` :!event `EnemyDeath`))
      ;[1 1 1] Adds to enemy list array
      (`KismetArrayLibrary.Array_Add` (`self.Enemy List`) _returnvalue))
    (:`NewEnumerator1`
      (bind _returnvalue_2 (`|SpawnActorFromClass` "/Game/Blueprints/AI/Characters/BP_BaseRanged.BP_BaseRanged_C" (`local.Local Transform`) "Undefined" "OverrideRootScale" null null))
      (add `self.OnDestroyed` _returnvalue_2 (`|CreateDelegate` :!event `EnemyDeath`))
      (`KismetArrayLibrary.Array_Add` (`self.Enemy List`) _returnvalue_2))
    (:`NewEnumerator2`
      (bind _returnvalue_3 (`|SpawnActorFromClass` "/Game/Blueprints/AI/Characters/BP_BaseMelee.BP_BaseMelee_C" (`local.Local Transform`) "Undefined" "OverrideRootScale" null null))
      (add `self.OnDestroyed` _returnvalue_3 (`|CreateDelegate` :!event `EnemyDeath`))
      (`KismetArrayLibrary.Array_Add` (`self.Enemy List`) _returnvalue_3))))

(fn `UserConstructionScript`)
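; Player character with melee attack toward stick or mouse, evade, interaction, damage and respawn at its start point, using a separately spawned camera and a basic HUD.
; Stats load from a data table on construction and supply the curves for attack and evade lunge timelines.
; Input during either action is queued for replay afterwards.
; Pickups grant permanent stat upgrades or a held speed buff; damage-over-time is an unwired stub.
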(event `self.ReceiveBeginPlay`
  ;[1 1 1] Camera Setup (for now...)
  (bind _returnvalue (`|SpawnActorFromClass` "/Game/Blueprints/Pawn/Pawn_Camera.Pawn_Camera_C" (`self.GetTransform`) "Undefined" "OverrideRootScale" null self null))
  (bind _output_get (set `self.Pawn_Camera` _returnvalue))
  (`PlayerController.SetViewTargetWithBlend` (`GameplayStatics.GetPlayerController` 0) _output_get 0.0 "VTBlend_Linear" 0.0 false)
  (`self.SetTimelineProperties` (`self.AttackMovement`) (`.AttackForwardCurve_39_77BCE8404CD50DAF7AC611A7AAF5505C` (break `/Game/Blueprints/Data/S_PlayerStats` (`self.PlayerStats`))))
  (`self.SetTimelineProperties` (`self.EvadeMovement`) (`.EvadeForwardCurve_37_BB76C5954F4C10B4EBDD0EA5FCEA0661` (break `/Game/Blueprints/Data/S_PlayerStats` (`self.PlayerStats`))))
  (bind _returnvalue_2 (`|CreateWidget` "/Game/Blueprints/UI/Widget_BasicHUD.Widget_BasicHUD_C"))
  (`UserWidget.AddToViewport` _returnvalue_2 0)
  (set `self.RespawnLocation` (`self.K2_GetActorLocation`)))

(event `AttackAnimation`
  ;[1 1 1] Attack Animation
  (bind _notifyname (`|PlayMontage` (`self.Mesh`) "/Game/CloseCombat/AM_PlayerAttackAttack.AM_PlayerAttackAttack" (`.MeleeAttackSpeed_28_9A8A8E9C42EC0FE283BCFF9DF5D00FEB` (break `/Game/Blueprints/Data/S_PlayerStats` (`self.PlayerStats`))))
    (:`OnCompleted`
      (if (`self.QueuedInput?`)
        (`self.InputQueue`)))
    (:`OnNotifyBegin`
      (if (== _notifyname "MoveForward")
        (bind _output_get (set `self.StartLocation` (`self.K2_GetActorLocation`)))
        (set `self.TargetLocation` (+ _output_get (* (`SceneComponent.GetForwardVector` (`self.Rotation`)) (`.AttackForwardDistance_30_F3D121124DBF3CE22A1F9B8CB4DDFC06` (break `/Game/Blueprints/Data/S_PlayerStats` (`self.PlayerStats`))))))
        (bind (_direction _alpha) (`Timeline|AttackMovement` :!via `PlayFromStart`)
          (:`Update`
            (`self.K2_SetActorLocation` (`KismetMathLibrary.VLerp` (`self.StartLocation`) (`self.TargetLocation`) _alpha) true))
          (:`Finished`
            (`KismetSystemLibrary.Delay` (`self.AttackResetTime`))
            (set `self.Attacking` false)))))))

(event `self.I_MouseAttack`
  ;[1 1 1] Mouse Attack
  (`self.IsThePlayerAlreadyAttackingEvading`
    (:`Yes`
      (set `self.QueuedInput?` true)
      (set `self.InputState` "NewEnumerator2"))
    (:`No`
      (set `self.Attacking` true)
      (set `self.QueuedInput?` false)
      (bind _outhit (`self.GetMouseLocationInWorld` (`self.MouseLocation`) (`self.MouseDirection`)))
      (`self.K2_SetActorRotation` (`KismetMathLibrary.MakeRotator` 0.0 0.0 (.yaw (`KismetMathLibrary.FindLookAtRotation` (`self.K2_GetActorLocation`) (`.Location` (`GameplayStatics.BreakHitResult` _outhit))))))
      (`self.AttackAnimation`))))

(event `InputQueue`
  (switch `/Game/Enums/EInputState` (`self.InputState`)
    (:`NewEnumerator0`
      (`self.I_Attack`))
    (:`NewEnumerator1`
      (`self.I_Evade`))
    (:`NewEnumerator2`
      (`self.I_MouseAttack`))))

(event `self.I_Attack`
  (bind _x_input (`self.X_Input`))
  (bind _y_input (`self.Y_Input`))
  ;[1 1 1] Attack
  (`self.IsThePlayerAlreadyAttackingEvading`
    (:`Yes`
      (set `self.QueuedInput?` true)
      (set `self.InputState` "NewEnumerator0"))
    (:`No`
      (set `self.Attacking` true)
      (set `self.QueuedInput?` false)
      (`self.IsThereNoLeftStickInput?` _x_input _y_input
        (:`Yes`
          (`self.K2_SetActorRotation` (`KismetMathLibrary.Conv_VectorToRotator` (`KismetMathLibrary.MakeVector` _x_input _y_input))))
        (:`No`
          _))
      (`self.AttackAnimation`))))

(event `self.I_Interact`
  ;[1 1 1] Interact with object
  (message `/Game/Blueprints/Interfaces/PickupInterface.PickedUp` (`PrimitiveComponent.GetOverlappingActors` (`self.CapsuleComponent`) null) self))

(event `/Game/Blueprints/Interfaces/I_Damageable.Damage`
  (params (Damage :type "Float (single-precision)") (KnockBack :type "Float (single-precision)") (InterfacingActor :type "Actor Object Reference"))
  (bind ((`Health_6_F6CC64834619DF6945EC6F8AE888027C` _health) (`MovementAcceleration_45_C1CE188B4266E168FC2CB7A569809289` _movementacceleration) (`MaxHP_25_7DEA515A4573369510A0DF9CE70A1188` _maxhp)) (break `/Game/Blueprints/Data/S_PlayerStats` (`self.PlayerStats`)))
  ;[1 1 1] Damage event for player
  (bind _structout (setmembers `/Game/Blueprints/Data/S_PlayerStats` :`StructRef` (`self.PlayerStats`) :`Health` (`KismetMathLibrary.FClamp` (- _health Damage) 0.0 _maxhp)))
  (if (<= (`.Health_6_F6CC64834619DF6945EC6F8AE888027C` (break `/Game/Blueprints/Data/S_PlayerStats` _structout)) 0.0)
    (`self.Death`)))

(event `self.I_UpDown`
  (params (Axis :type "Float (single-precision)"))
  ;[1 1 1] Move Character
  (set `self.Y_Input` Axis)
  (`PawnMovementComponent.AddInputVector` (`self.CharacterMovement`) (`KismetMathLibrary.MakeVector` (stale `self.I_LeftRight` Axis) Axis) false :!label _label))

(event `self.I_LeftRight`
  (params (Axis :type "Float (single-precision)"))
  ;[1 1 1] Move Character
  (set `self.X_Input` Axis)
  (goto _label))

(event `self.I_Evade`
  (bind _returnvalue (`self.K2_GetActorLocation`))
  ;[1 1 1] Evade
  (`self.IsThePlayerAlreadyAttackingEvading`
    (:`Yes`
      (set `self.QueuedInput?` true)
      (set `self.InputState` "NewEnumerator1"))
    (:`No`
      (set `self.Evading` true)
      (set `self.QueuedInput?` false)
      (`self.IsThereNoLeftStickInput?` (`self.X_Input`) (`self.Y_Input`)
        (:`Yes`
          (`self.K2_SetActorRotation` (`KismetMathLibrary.Conv_VectorToRotator` (`KismetMathLibrary.MakeVector` (`self.X_Input`) (`self.Y_Input`)))))
        (:`No`
          _))
      (set `self.StartLocation` _returnvalue)
      (set `self.TargetLocation` (+ _returnvalue (* (`SceneComponent.GetForwardVector` (`self.Rotation`)) (`.EvadeForwardDistance_32_2EB0C1D149E2460604C01A8F1356CEC0` (break `/Game/Blueprints/Data/S_PlayerStats` (`self.PlayerStats`))))))
      (bind (_direction _alpha) (`Timeline|EvadeMovement` :!via `PlayFromStart`)
        (:`Update`
          (`self.K2_SetActorLocation` (`KismetMathLibrary.VLerp` (`self.StartLocation`) (`self.TargetLocation`) _alpha) true))
        (:`Finished`
          (set `self.Evading` false)
          (if (`self.QueuedInput?`)
            (`self.InputQueue`)))))))

(event `Death`
  ;[1 1 1] Death and respawn
  (`KismetSystemLibrary.Delay` 0.2)
  (`self.Respawn`))

(event `self.ReceiveTick`
  (params (DeltaSeconds :type "Float (single-precision)"))
  (bind (_worldlocation _worlddirection) (`PlayerController.DeprojectMousePositionToWorld` (`GameplayStatics.GetPlayerController` 0)))
  ;[1 1 1] Get Mouse Location
  (set `self.MouseLocation` _worldlocation)
  (set `self.MouseDirection` _worlddirection))

(event `Respawn`
  ;[1 1 1] Death and respawn
  (setmembers `/Game/Blueprints/Data/S_PlayerStats` :`StructRef` (`self.PlayerStats`) :`Health` (`.MaxHP_25_7DEA515A4573369510A0DF9CE70A1188` (break `/Game/Blueprints/Data/S_PlayerStats` (`self.PlayerStats`))))
  (`self.K2_SetActorLocation` (`self.RespawnLocation`)))

(event `AddBuff`
  (params (NewBuff :type String))
  (bind _charactermovement (`self.CharacterMovement`))
  (bind _charactermovement_2 (`self.CharacterMovement`))
  ;[1 1 1] Very messy implementation of holdable buffs
  (if (not (`KismetStringLibrary.EqualEqual_StrStr` (`self.CurrentBuff`) "EmptyBuff"))
    (bind _returnvalue (`|GetDataTableRow` "/Game/Blueprints/Data/DT_Pickups.DT_Pickups" (`KismetStringLibrary.Conv_StringToName` (`self.CurrentBuff`)))
      (:`then`
        (bind ((`Stat_14_4AE0A22B417522BD605BB9AEE66F9DBF` _stat) (`PotencyStrength_11_731EB910491EB27E32DD7F9C01E345C7` _potencystrength)) (break `/Game/Blueprints/Data/S_Pickup` _returnvalue))
        (bind _result (`/Engine/EditorBlueprintResources/StandardMacros.NegateFloat` _potencystrength)
          (:`  `
            (switch `string` _stat
              (:`Speed`
                (set `CharacterMovementComponent.MaxWalkSpeed` (+ (`CharacterMovementComponent.MaxWalkSpeed` _charactermovement) _result) _charactermovement))))))))
  (bind _returnvalue_2 (`|GetDataTableRow` "/Game/Blueprints/Data/DT_Pickups.DT_Pickups" (`KismetStringLibrary.Conv_StringToName` NewBuff))
    (:`then`
      (bind ((`Stat_14_4AE0A22B417522BD605BB9AEE66F9DBF` _stat_2) (`PotencyStrength_11_731EB910491EB27E32DD7F9C01E345C7` _potencystrength_2)) (break `/Game/Blueprints/Data/S_Pickup` _returnvalue_2))
      (switch `string` _stat_2
        (:`Speed`
          (set `CharacterMovementComponent.MaxWalkSpeed` (+ (`CharacterMovementComponent.MaxWalkSpeed` _charactermovement_2) _potencystrength_2) _charactermovement_2)
          (set `self.CurrentBuff` NewBuff))))))

(event `Ticking Effect Example`
  (params (Time :type "Float (double-precision)") (Value :type "Float (double-precision)"))
  ;[1 1 1] Dot Event
)

(event `/Game/Blueprints/Interfaces/I_Upgrade.I_Upgrade`
  (params (UpgradeEffect :type "/Game/Blueprints/Data/S_Upgrades Structure"))
  ;[1 1 1] Upgrades
  (if (not (`.Temporary_1_55C9E60041C20CBBCCC2BF8F3FAB51ED` (break `/Game/Blueprints/Data/S_Upgrades` UpgradeEffect)))
    (`self.PermanentUpgrade` UpgradeEffect)))

(fn `ChangeAOEDamage`
  (params (Change :type "Float (double-precision)"))
  (setmembers `/Game/Blueprints/Data/S_PlayerStats` :`StructRef` (`self.PlayerStats`) :`AOE Damage` (+ Change (`.AOEDamage_15_FB13F3B64A4952C5C74A6CBEA72BEC6F` (break `/Game/Blueprints/Data/S_PlayerStats` (`self.PlayerStats`))))))

(fn `ChangeMeleeDamage`
  (params (Change :type "Float (double-precision)"))
  (setmembers `/Game/Blueprints/Data/S_PlayerStats` :`StructRef` (`self.PlayerStats`) :`MeleeDamage` (+ Change (`.MeleeDamage_10_29F022B343CE9AC80872E2B63DB99040` (break `/Game/Blueprints/Data/S_PlayerStats` (`self.PlayerStats`))))))

(fn `ChangeMeleeSpeed`
  (params (Change :type "Float (double-precision)"))
  (setmembers `/Game/Blueprints/Data/S_PlayerStats` :`StructRef` (`self.PlayerStats`) :`MeleeAttackSpeed` (+ Change (`.MeleeAttackSpeed_28_9A8A8E9C42EC0FE283BCFF9DF5D00FEB` (break `/Game/Blueprints/Data/S_PlayerStats` (`self.PlayerStats`))))))

(fn `ChangeSpellDamage`
  (params (Change :type "Float (double-precision)"))
  (setmembers `/Game/Blueprints/Data/S_PlayerStats` :`StructRef` (`self.PlayerStats`) :`SpellDamage` (+ Change (`.SpellDamage_19_975A20A14D26CBAAC5D0268ECCBDB818` (break `/Game/Blueprints/Data/S_PlayerStats` (`self.PlayerStats`))))))

(fn `ChangeStunningAttack`
  (params (Change :type "Float (double-precision)"))
  (if (>= Change 1.0)
    (setmembers `/Game/Blueprints/Data/S_PlayerStats` :`StructRef` (`self.PlayerStats`) :`Stunning Attack` true)))

(fn `DamageOverTime`
  (`KismetSystemLibrary.PrintString` "Dot Event"))

(fn `GetMouseLocationInWorld`
  (params (Location :type "Vector Structure") (Direction :type "Vector Structure"))
  (returns (OutHit :type "HitResult Structure"))
  (bind _outhit (`KismetSystemLibrary.LineTraceSingle` :`Start` Location :`End` (+ Location (* (* Direction (/ (.z Location) (.z Direction))) -2.0)) :`TraceChannel` "TraceTypeQuery1" :`DrawDebugType` "ForDuration"))
  (return _outhit))

(fn `I_GetMesh`
  (returns (SkeletalMesh :type "SkeletalMeshComponent Object Reference"))
  (return null))

(fn `I_GetTeam`
  (returns (ETeam :type "/Game/Enums/ETeam Enum"))
  (return (`self.ETeam`)))

(fn `I_GetWeaponEquipped`
  (returns (WeaponEquipped :type "Actor Object Reference"))
  (return (`ChildActorComponent.ChildActor` (`self.Weapon`))))

(fn `PermanentUpgrade`
  (params (Pickup :type "/Game/Blueprints/Data/S_Upgrades Structure"))
  (locals (LocalPotency :type "Float (double-precision)"))
  (bind ((`Stat_14_4AE0A22B417522BD605BB9AEE66F9DBF` _stat) (`PotencyStrength_11_731EB910491EB27E32DD7F9C01E345C7` _potencystrength)) (break `/Game/Blueprints/Data/S_Upgrades` Pickup))
  ;[1 1 1] Takes Pickup Information and switches to buff different stat based on type
  (set `local.LocalPotency` _potencystrength)
  (switch `string` _stat
    (:`MeleeDamage`
      (`self.ChangeMeleeDamage` (`local.LocalPotency`)))
    (:`AttackSpeed`
      (`self.ChangeMeleeSpeed` (`local.LocalPotency`)))
    (:`StunningAttackBuff`
      (`self.ChangeStunningAttack` (`local.LocalPotency`)))
    (:`AOEDamage`
      (`self.ChangeAOEDamage` (`local.LocalPotency`)))
    (:`SpellDamageBuff`
      (`self.ChangeSpellDamage` (`local.LocalPotency`)))))

(fn `SetTimelineProperties`
  (params (Timeline :type "TimelineComponent Object Reference") (NewFloatCurve :type "CurveFloat Object Reference"))
  (`TimelineComponent.SetFloatCurve` Timeline NewFloatCurve "Alpha")
  (`TimelineComponent.SetTimelineLength` Timeline (`.MaxTime` (`CurveBase.GetTimeRange` NewFloatCurve))))

(fn `UserConstructionScript`
  (`SceneComponent.K2_AttachToComponent` (`self.Weapon`) (`self.Mesh`) "Socket_Weapon" "KeepRelative" "KeepRelative" "KeepRelative" true)
  (bind _returnvalue (`|GetDataTableRow` "/Game/Blueprints/Data/DT_PlayerStats.DT_PlayerStats" "Iter1")
    (:`then`
      (bind _output_get (set `self.PlayerStats` _returnvalue))
      (bind (_health _movespeed _movementacceleration _meleedamage _aoedamage _spelldamage _stunningattack _maxhp _meleeattackspeed _attackforwarddistance _attackforwardcurve _evadeforwarddistance _evadeforwardcurve _rotationrate) (break `/Game/Blueprints/Data/S_PlayerStats` _output_get))
      (set `CharacterMovementComponent.MaxWalkSpeed` _movespeed (`self.CharacterMovement`))
      (bind _asbp_player_weapon (cast `/Game/Blueprints/Weapon/BP_PlayerWeapon` (`ChildActorComponent.ChildActor` (`self.Weapon`))))
      (set `/Game/Blueprints/Weapon/BP_BaseWeapon.Damage` _meleedamage _asbp_player_weapon)
      (set `CharacterMovementComponent.RotationRate` _rotationrate (`self.CharacterMovement`))
      (set `CharacterMovementComponent.MaxAcceleration` _movementacceleration (`self.CharacterMovement`)))))
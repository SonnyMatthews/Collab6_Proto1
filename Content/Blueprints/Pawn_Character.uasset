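; Player character pawn that moves, attacks and evades through interface events, spawning its own camera actor on BeginPlay.
; Attack and evade snap facing to stored stick input, then lerp the actor forward on timelines whose curve and length are set at runtime.
; DoOnce gates block repeats: attack resets when its lunge ends, toggling the child-actor weapon around it, while evade resets after a cooldown delay.
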(event `self.ReceiveBeginPlay`
  ;[1 1 1] Camera Setup (for now...)
  (bind _returnvalue (`|SpawnActorFromClass` "/Game/Blueprints/Pawn_Camera.Pawn_Camera_C" (`self.GetTransform`) "Undefined" "OverrideRootScale" null self null))
  (`PlayerController.SetViewTargetWithBlend` (`GameplayStatics.GetPlayerController` 0) _returnvalue 0.0 "VTBlend_Linear" 0.0 false))

(event `/Game/Blueprints/I_Controller.I_Attack`
  (bind (_returnvalue_x _returnvalue_y _returnvalue_z) (`KismetMathLibrary.BreakVector` (`self.K2_GetActorLocation`)))
  (bind _y_input (`self.Y_Input`))
  (bind _x_input (`self.X_Input`))
  ;[1 1 1] Attack
  (`/Engine/EditorBlueprintResources/StandardMacros.DoOnce` false :!label _label
    (:`Completed`
      (`self.IsThereNoLeftStickInput?` _y_input _x_input
        (:`Yes`
          (`self.K2_SetActorRotation` (`KismetMathLibrary.Conv_VectorToRotator` (`KismetMathLibrary.MakeVector` _y_input _x_input 0.0))))
        (:`No`
          _))
      (bind _output_get (set `self.StartLocation` (`self.K2_GetActorLocation`)))
      (set `self.TargetLocation` (+ _output_get (* (`SceneComponent.GetForwardVector` (`self.Rotation`)) (`self.AttackDistance`))))
      (message `/Game/Blueprints/I_Weapon.I_ActivateWeapon` (`ChildActorComponent.ChildActor` (`self.Weapon`)))
      (`self.SetTimelineProperties` (`self.AttackMovement`) (`self.AttackMovementCurve`))
      (bind (_direction _alpha) (`Timeline|AttackMovement` :!via `PlayFromStart`)
        (:`Update`
          (bind (_returnvalue_x_2 _returnvalue_y_2) (`KismetMathLibrary.BreakVector` (`KismetMathLibrary.VLerp` (`self.StartLocation`) (`self.TargetLocation`) _alpha)))
          (`self.K2_SetActorLocation` (`KismetMathLibrary.MakeVector` _returnvalue_x_2 _returnvalue_y_2 _returnvalue_z)))
        (:`Finished`
          (message `/Game/Blueprints/I_Weapon.I_DeactivateWeapon` (`ChildActorComponent.ChildActor` (`self.Weapon`)))
          (`self.ResetAttack`))))))

(event `ResetAttack`
  ;[1 1 1] Attack
  (goto _label :!via `Reset`))

(event `/Game/Blueprints/I_Controller.I_UpDown`
  (params (Axis :type "Float (single-precision)"))
  ;[1 1 1] Move Character
  (set `self.X_Input` Axis)
  (`PawnMovementComponent.AddInputVector` (`self.CharacterMovement`) (`KismetMathLibrary.MakeVector` (stale `/Game/Blueprints/I_Controller.I_LeftRight` Axis) Axis) false :!label _label_2))

(event `/Game/Blueprints/I_Controller.I_LeftRight`
  (params (Axis :type "Float (single-precision)"))
  ;[1 1 1] Move Character
  (set `self.Y_Input` Axis)
  (goto _label_2))

(event `/Game/Blueprints/I_Controller.I_Evade`
  (bind _returnvalue (`self.K2_GetActorLocation`))
  ;[1 1 1] Evade
  (`/Engine/EditorBlueprintResources/StandardMacros.DoOnce` false :!label _label_3
    (:`Completed`
      (`self.IsThereNoLeftStickInput?` (`self.Y_Input`) (`self.X_Input`)
        (:`Yes`
          (`self.K2_SetActorRotation` (`KismetMathLibrary.Conv_VectorToRotator` (`KismetMathLibrary.MakeVector` (`self.Y_Input`) (`self.X_Input`)))))
        (:`No`
          _))
      (set `self.StartLocation` _returnvalue)
      (set `self.TargetLocation` (+ _returnvalue (* (`SceneComponent.GetForwardVector` (`self.Rotation`)) (`self.EvadeDistance`))))
      (`self.SetTimelineProperties` (`self.EvadeMovement`) (`self.EvadeMovementCurve`))
      (bind (_direction _alpha) (`Timeline|EvadeMovement` :!via `PlayFromStart`)
        (:`Update`
          (`self.K2_SetActorLocation` (`KismetMathLibrary.VLerp` (`self.StartLocation`) (`self.TargetLocation`) _alpha)))
        (:`Finished`
          (`KismetSystemLibrary.Delay` (`self.DashResetTime`))
          (`self.Reset Dash`))))))

(event `Reset Dash`
  ;[1 1 1] Evade
  (goto _label_3 :!via `Reset`))

(event `self.ReceiveTick`
  (params (DeltaSeconds :type "Float (single-precision)"))
  ;[1 1 1] Speed
)

(fn `SetTimelineProperties`
  (params (Timeline :type "TimelineComponent Object Reference") (NewFloatCurve :type "CurveFloat Object Reference"))
  (`TimelineComponent.SetFloatCurve` Timeline NewFloatCurve "Alpha")
  (`TimelineComponent.SetTimelineLength` Timeline (`.MaxTime` (`CurveBase.GetTimeRange` NewFloatCurve))))

(fn `UserConstructionScript`)
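; Base pickup actor that grants a named buff to the actor passed to PickedUp, guarded by a DoOnce.
; PickupType then destroys it or hides it and disables collision, with a respawn timer only for the timed type.
; Reactivate plays an effect and sound, briefly delays, then resets the DoOnce and restores collision and visibility.
; TimerActivate starts the pickup hidden on that timer; nothing here reactivates Respawn on Death pickups.
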(event `self.ReceiveBeginPlay`
  (if (`self.TimerActivate?`)
    (`self.Deactivate` true)))

(event `/Game/Blueprints/Interfaces/PickupInterface.PickedUp`
  (params (Actor :type "/Game/Blueprints/Pawn/Pawn_Character Object Reference"))
  ;[1 1 1] call function in player to replace or set a buff
  (`KismetSystemLibrary.PrintString` "Picked up")
  (`/Engine/EditorBlueprintResources/StandardMacros.DoOnce` false :!label _label
    (:`Completed`
      (`/Game/Blueprints/Pawn/Pawn_Character.AddBuff` Actor (`|GetEnumeratorNameAsString` (`self.BuffName`)))
      ;[1 1 1] Deactivate in way based on inputs
      (switch `/Game/Enums/PickupRespawnTypes` (`self.PickupType`)
        (:`NewEnumerator0`
          (`self.K2_DestroyActor`))
        (:`NewEnumerator1`
          (`self.Deactivate` false))
        (:`NewEnumerator2`
          (`self.Deactivate` true))))))

(event `Reactivate`
  (bind _returnvalue (`self.K2_GetActorLocation`))
  (bind _staticmesh (`self.StaticMesh`))
  ;[1 1 1] For pickups that respawn over time
  (`GameplayStatics.SpawnEmitterAtLocation` null _returnvalue)
  (`GameplayStatics.PlaySoundAtLocation` null _returnvalue (struct) 1.0 1.0 0.0 null null null)
  (`KismetSystemLibrary.Delay` 0.4)
  (`|ExecutionSequence`
    (:`then_0`
      (goto _label :!via `Reset`))
    (:`then_1`
      (`PrimitiveComponent.SetCollisionEnabled` (`self.SphereCollision`) "QueryOnly")
      (`/Engine/EditorBlueprintResources/StandardMacros.IsValid` _staticmesh
        (:`Is Valid`
          (`SceneComponent.SetVisibility` _staticmesh true false))))))

(event `Deactivate`
  (params (UsingTimer :type Boolean))
  ;[1 1 1] For pickups that respawn over time
  (if UsingTimer
    (`KismetSystemLibrary.K2_SetTimerDelegate` (delegate `Reactivate`) (`self.RespawnTime`)))
  (`PrimitiveComponent.SetCollisionEnabled` (`self.SphereCollision`) "NoCollision")
  (`SceneComponent.SetVisibility` (`self.StaticMesh`) false false))

(fn `UserConstructionScript`)
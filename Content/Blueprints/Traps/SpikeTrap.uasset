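; Spike trap actor that deals damage with zero knockback to overlapping actors.
; Begin overlap damages the entering actor at once and starts a looping ReactTime timer for ShootSpikes.
; ShootSpikes stores the box's BP_BaseMelee overlaps in ActorsToHit, appends that to a separate Pawn_Character query result, then damages only ActorsToHit.
; End overlap clears the timer only when the last stored ActorsToHit is empty; RetractTime is unused.
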(event `self.ReceiveActorBeginOverlap`
  (params (OtherActor :type "Actor Object Reference"))
  (message `/Game/Blueprints/Interfaces/I_Damageable.Damage` OtherActor (`self.Damage`) 0.0 null)
  (bind _returnvalue (`KismetSystemLibrary.K2_SetTimerDelegate` (delegate `ShootSpikes`) (`self.ReactTime`) true))
  (set `self.HitTimer` _returnvalue))

(event `ShootSpikes`
  (bind _box (`self.Box`))
  (bind _output_get (set `self.ActorsToHit` (`PrimitiveComponent.GetOverlappingActors` _box "/Game/Blueprints/AI/Characters/BP_BaseMelee.BP_BaseMelee_C")))
  (`KismetArrayLibrary.Array_Append` (`PrimitiveComponent.GetOverlappingActors` _box "/Game/Blueprints/Pawn/Pawn_Character.Pawn_Character_C") _output_get)
  (for _array_element (`self.ActorsToHit`)
    (message `/Game/Blueprints/Interfaces/I_Damageable.Damage` _array_element (`self.Damage`) 0.0 null)
    (`KismetSystemLibrary.PrintString` "Damaged something")))

(event `self.ReceiveActorEndOverlap`
  (params (OtherActor :type "Actor Object Reference"))
  (if (not (`KismetArrayLibrary.Array_IsValidIndex` (`self.ActorsToHit`)))
    (`KismetSystemLibrary.K2_ClearAndInvalidateTimerHandle` (`self.HitTimer`))))

(fn `UserConstructionScript`)
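; BP_Pickup_Buff is a child pickup Blueprint that hands a buff's stats to the actor that overlaps it.
; SetPickup loads PickupStats from the DT_Pickups data table, using the PickupType enum's name as the row key.
; PickupEffect passes those stats to the overlapped actor through the IUpgradeMessage interface call.
; Both functions replace their parent versions without calling them, and the event graph holds only disabled stubs.
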(fn `PickupEffect`
  (params (Overlapped :type "Actor Object Reference"))
  (message `/Game/Blueprints/Upgrades/I_Pickup.I_Upgrade` Overlapped (`self.PickupStats`)))

(fn `SetPickup`
  (bind _returnvalue (`|GetDataTableRow` "/Game/Blueprints/Upgrades/DT_Pickups.DT_Pickups" (`|GetEnumeratorName` (`self.PickupType`)))
    (:`then`
      (set `self.PickupStats` _returnvalue))))

(fn `UserConstructionScript`
  (`parent.UserConstructionScript`))
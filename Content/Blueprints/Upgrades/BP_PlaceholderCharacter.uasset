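; Placeholder character that receives pickup upgrades through the IUpgrade interface and applies them to its PlayerStats struct.
; Pickups route to permanent or temporary handlers, which switch on stat to adjust melee, attack speed, AOE or spell damage.
; Temporary buffs reverse after a Delay using shared potency variables; stunning attack is permanent-only.
; An example ticking effect starts a looping timer that drains Health, with no timer clear after its Delay.
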(event `/Game/Blueprints/Interfaces/I_Upgrade.I_Upgrade`
  (params (PickupEffect :type "/Game/Blueprints/Data/S_Pickup Structure"))
  (if (`.Temporary_1_55C9E60041C20CBBCCC2BF8F3FAB51ED` (break `/Game/Blueprints/Data/S_Pickup` PickupEffect))
    (`self.TempUpgrade` PickupEffect)
    (else
      (`self.Perm Upgrade` PickupEffect))))

(event `TempUpgrade`
  (params (PickupEffect :type "/Game/Blueprints/Data/S_Pickup Structure"))
  (bind ((`Stat_14_4AE0A22B417522BD605BB9AEE66F9DBF` _stat) (`Time_10_75ED92B349EF05A1F51D54B2411CB5FB` _time) (`PotencyStrength_11_731EB910491EB27E32DD7F9C01E345C7` _potencystrength)) (break `/Game/Blueprints/Data/S_Pickup` PickupEffect))
  ;[1 1 1] Changes Value, then after a delay removes same amount
  (set `self.BuffTime` _time)
  (set `self.Buff Potency` _potencystrength)
  (switch `string` _stat
    (:`MeleeDamage`
      (`self.ChangeMeleeDamage` (`self.Buff Potency`))
      (`KismetSystemLibrary.Delay` (`self.BuffTime`))
      (`self.ChangeMeleeDamage` (* (`self.Buff Potency`) -1.0)))
    (:`AttackSpeed`
      (`self.ChangeMeleeAttackSpeed` (`self.Buff Potency`))
      (`KismetSystemLibrary.Delay` (`self.BuffTime`))
      (`self.ChangeMeleeAttackSpeed` (* (`self.Buff Potency`) -1.0)))
    (:`AOEDamage`
      (`self.ChangeAoeDamage` (`self.Buff Potency`))
      (`KismetSystemLibrary.Delay` (`self.BuffTime`))
      (`self.ChangeAoeDamage` (* (`self.Buff Potency`) -1.0)))
    (:`SpellDamageBuff`
      (`self.ChangeRangedDamage` (`self.Buff Potency`))
      (`KismetSystemLibrary.Delay` (`self.BuffTime`))
      (`self.ChangeRangedDamage` (* (`self.Buff Potency`) -1.0)))))

(event `Ticking Effect Example`
  (params (Time :type "Float (double-precision)") (Value :type "Float (double-precision)"))
  (set `self.BurnDmg` Value)
  (bind _returnvalue (`KismetSystemLibrary.K2_SetTimer` self "Burning" 1.0 true))
  (set `self.BurningHandle` _returnvalue)
  (`KismetSystemLibrary.Delay` Time))

(fn `Burning`
  (setmembers `/Game/Blueprints/Data/S_PlayerStats` :`StructRef` (`self.PlayerStats`) :`Health` (- (`.Health_6_F6CC64834619DF6945EC6F8AE888027C` (break `/Game/Blueprints/Data/S_PlayerStats` (`self.PlayerStats`))) (`self.BurnDmg`))))

(fn `ChangeAoeDamage`
  (params (DamageChange :type "Float (double-precision)"))
  (setmembers `/Game/Blueprints/Data/S_PlayerStats` :`StructRef` (`self.PlayerStats`) :`AOE Damage` (+ DamageChange (`.AOEDamage_15_FB13F3B64A4952C5C74A6CBEA72BEC6F` (break `/Game/Blueprints/Data/S_PlayerStats` (`self.PlayerStats`))))))

(fn `ChangeMeleeAttackSpeed`
  (params (ValueChange :type "Float (double-precision)"))
  (locals (TempPickupStats :type "/Game/Blueprints/Data/S_Pickup Structure"))
  (setmembers `/Game/Blueprints/Data/S_PlayerStats` :`StructRef` (`self.PlayerStats`) :`MeleeAttackSpeed` (+ ValueChange (`.MeleeAttackSpeed_11_5238446041BFD0477CB012B1A4A9B1BF` (break `/Game/Blueprints/Data/S_PlayerStats` (`self.PlayerStats`))))))

(fn `ChangeMeleeDamage`
  (params (DamageChange :type "Float (double-precision)"))
  (locals (TempPickupStats :type "/Game/Blueprints/Data/S_Pickup Structure"))
  (setmembers `/Game/Blueprints/Data/S_PlayerStats` :`StructRef` (`self.PlayerStats`) :`MeleeDamage` (+ DamageChange (`.MeleeDamage_10_29F022B343CE9AC80872E2B63DB99040` (break `/Game/Blueprints/Data/S_PlayerStats` (`self.PlayerStats`))))))

(fn `ChangeRangedDamage`
  (params (DamageChange :type "Float (double-precision)"))
  (setmembers `/Game/Blueprints/Data/S_PlayerStats` :`StructRef` (`self.PlayerStats`) :`SpellDamage` (+ DamageChange (`.SpellDamage_19_975A20A14D26CBAAC5D0268ECCBDB818` (break `/Game/Blueprints/Data/S_PlayerStats` (`self.PlayerStats`))))))

(fn `ChangeToStunningAttack`
  (params (DamageChange :type "Float (double-precision)"))
  (if (>= DamageChange 1.0)
    (setmembers `/Game/Blueprints/Data/S_PlayerStats` :`StructRef` (`self.PlayerStats`) :`Stunning Attack` true)))

(fn `Perm Upgrade`
  (params (S_Pickup :type "/Game/Blueprints/Data/S_Pickup Structure (by ref)"))
  (locals (LocalPotency :type "Float (double-precision)"))
  (bind ((`Stat_14_4AE0A22B417522BD605BB9AEE66F9DBF` _stat) (`PotencyStrength_11_731EB910491EB27E32DD7F9C01E345C7` _potencystrength)) (break `/Game/Blueprints/Data/S_Pickup` S_Pickup))
  (set `local.LocalPotency` _potencystrength)
  (switch `string` _stat
    (:`MeleeDamage`
      (`self.ChangeMeleeDamage` (`local.LocalPotency`)))
    (:`AttackSpeed`
      (`self.ChangeMeleeAttackSpeed` (`local.LocalPotency`)))
    (:`StunningAttackBuff`
      (`self.ChangeToStunningAttack` (`local.LocalPotency`)))
    (:`AOEDamage`
      (`self.ChangeAoeDamage` (`local.LocalPotency`)))
    (:`SpellDamageBuff`
      (`self.ChangeRangedDamage` (`local.LocalPotency`)))))

(fn `UserConstructionScript`)
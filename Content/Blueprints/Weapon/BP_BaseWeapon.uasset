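; BP_BaseWeapon is a base weapon actor that deals damage through a box hitbox.
; Interface events show and enable the box for an attack window, then hide and disable it and clear the hit list.
; On overlap, it sends a damage message with zero knockback to actors carrying the target tag, excluding its parent actor.
; The HitActors list limits each target to one hit per activation.
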(event `/Game/Blueprints/Interfaces/I_Weapon.I_ActivateWeaponHitbox`
  ;[1 1 1] Hit Box Activation
  (`SceneComponent.SetVisibility` (`self.Box`) true false)
  (`PrimitiveComponent.SetCollisionEnabled` (`self.Box`) "QueryAndPhysics"))

(event `/Game/Blueprints/Interfaces/I_Weapon.I_DeactivateWeaponHitbox`
  ;[1 1 1] Hit Box Activation
  (`SceneComponent.SetVisibility` (`self.Box`) false false)
  (`PrimitiveComponent.SetCollisionEnabled` (`self.Box`) "NoCollision")
  (`KismetArrayLibrary.Array_Clear` (`self.HitActors`)))

(event `self.Box.OnComponentBeginOverlap`
  (params (OverlappedComponent :type "PrimitiveComponent Object Reference") (OtherActor :type "Actor Object Reference") (OtherComp :type "PrimitiveComponent Object Reference") (OtherBodyIndex :type Integer) (bFromSweep :type Boolean) (SweepResult :type "HitResult Structure (by ref)"))
  ;[1 1 1] Overlap
  (if (`KismetArrayLibrary.Array_Contains` (`self.HitActors`) OtherActor)
    _
    (elif (`self.ActorHasTag` OtherActor (`self.ActorToHitTag`))
      (if (not (== (`self.GetParentActor`) OtherActor))
        (`KismetArrayLibrary.Array_AddUnique` (`self.HitActors`) OtherActor)
        (message `/Game/Blueprints/Interfaces/I_Damageable.Damage` OtherActor (`self.Damage`) 0.0 self)))))

(fn `UserConstructionScript`)
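; Base projectile actor, filed under enemy weapons, that damages and knocks back what it overlaps.
; InitProjectile stores the owner, damage and knockback, sets the movement component's velocity from direction and speed, then flags the projectile as initialised.
; Once initialised, a collision sphere overlap with any non-owner implementing I_Damageable calls Damage with the owner as interfacing actor, then destroys the projectile.
; Overlaps with non-damageable actors leave it alive.
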(event `self.collisionSphere.OnComponentBeginOverlap`
  (params (OverlappedComponent :type "PrimitiveComponent Object Reference") (OtherActor :type "Actor Object Reference") (OtherComp :type "PrimitiveComponent Object Reference") (OtherBodyIndex :type Integer) (bFromSweep :type Boolean) (SweepResult :type "HitResult Structure (by ref)"))
  ;[1 1 1] On hit something add damaage
  (if (`self._initialised`)
    (if (!= OtherActor (`self._Owner`))
      (bind _asi_damageable (cast `/Game/Blueprints/Interfaces/I_Damageable` OtherActor))
      (`/Game/Blueprints/Interfaces/I_Damageable.Damage` _asi_damageable (`self._damage`) (`self._knockBack`) (`self._Owner`))
      (`self.K2_DestroyActor`))))

(fn `InitProjectile`
  (params (InitialSpeed :type "Float (double-precision)") (_knockBack :type "Float (double-precision)") (_damage :type "Float (double-precision)") (ProjectileOwner :type "Actor Object Reference") (direction :type "Vector Structure"))
  (locals (velocity :type "Vector Structure"))
  (set `self._Owner` ProjectileOwner)
  (set `self._knockBack` _knockBack)
  (set `self._damage` _damage)
  (bind _output_get (set `local.velocity` (* direction InitialSpeed)))
  (set `MovementComponent.Velocity` _output_get (`self.ProjectileMovement`))
  (set `self._initialised` true))

(fn `UserConstructionScript`)